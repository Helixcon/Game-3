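; Zombie spawner actor that spawns waves of AI from SpawnerStruct, starting shortly after BeginPlay unless UseOverlapToActivate is set.
; Each wave plays particle and sound effects, then spawns its enemies at random navigable points near SpawnLocation.
; A delayed polling loop starts the next wave once all spawned enemies are invalid; the spawner destroys itself after spawning the last.
; When enabled, custom depth is passed to spawned enemies.
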(event `/Game/ArcherySystem/Bow/BPI_BowPostProcess.EnableCustomDepth`
  ;[0 0 0 0.5] Enable custom depth, this is used to enable custom depth on the AI if the player has it enabled.
  (set `self.CustomDepthEnabled` true))

(event `/Game/ArcherySystem/Bow/BPI_BowPostProcess.DisableCustomDepth`
  ;[0 0 0 0.5] Enable custom depth, this is used to enable custom depth on the AI if the player has it enabled.
  (set `self.CustomDepthEnabled` false))

(event `MultiCastParticles`
  (bind _spawnparticlescale (`self.SpawnParticleScale`))
  (bind _returnvalue (`SceneComponent.K2_GetComponentLocation` (`self.DefaultSceneRoot`)))
  ;[0 0 0 0.5] Particle and sounds for when AI spawns.
  (`GameplayStatics.SpawnEmitterAtLocation` (`self.SpawnEmitter`) _returnvalue (struct) (`KismetMathLibrary.MakeVector` _spawnparticlescale _spawnparticlescale _spawnparticlescale))
  (`GameplayStatics.SpawnSoundAtLocation` "/Game/ArcherySystem/Assets/Sounds/Ambient/A_UI_WaveEnd_Cue.A_UI_WaveEnd_Cue" _returnvalue (struct) 1.0 1.0 0.0 null null))

(event `self.ReceiveBeginPlay`
  ;[0 0.4054 1] Beginplay (Spawn AI if there's no Overlap required)
  (if (not (`self.UseOverlapToActivate`))
    (`KismetSystemLibrary.Delay` 1.0)
    (`self.SpawnEnemies`)))

(event `SpawnEnemies`
  (bind _spawnlocation (`self.SpawnLocation`))
  (bind (_output_enemiestospawn _output_enemytospawn) (break `/Game/ArcherySystem/Blueprints/AI/Spawner/ST_Spawner` (`|GetArrayItem` (`self.SpawnerStruct`) (`self.ActiveStruct`))))
  (`|ExecutionSequence`
    (:`then_0`
      (`self.MultiCastParticles`))
    (:`then_1`
      ;[0 0 0] Spawn AI.
      (`KismetSystemLibrary.Delay` 0.2)
      (for _ (range _output_enemiestospawn)
        (bind _returnvalue (`AIBlueprintHelperLibrary.SpawnAIFromClass` _output_enemytospawn null (`NavigationSystemV1.K2_GetRandomLocationInNavigableRadius` (`SceneComponent.K2_GetComponentLocation` _spawnlocation) 150.0 null null) (`SceneComponent.K2_GetComponentRotation` _spawnlocation) false null))
        (`KismetArrayLibrary.Array_Add` (`self.SpawnedEnemies`) _returnvalue))
      ;[0 0 0 0.5] Check if there is another wave that needs to be spawned. (Once everyone is dead, a new wave will spawn, if there is no new wave, the actor will deleate itself)
      (`self.MultiCastCustomDepth` (`self.SpawnedEnemies`))
      (bind _result (`/Engine/EditorBlueprintResources/StandardMacros.IncrementInt` (`self.ActiveStruct`))
        (:`  `
          (if (`KismetArrayLibrary.Array_IsValidIndex` (`self.SpawnerStruct`) _result)
            (set `self.SpawnNewRound` false :!label _label)
            (for _array_element (`self.SpawnedEnemies`)
              (`/Engine/EditorBlueprintResources/StandardMacros.IsValid` _array_element
                (:`Is Valid`
                  (set `self.SpawnNewRound` true))))
            (if (`self.SpawnNewRound`)
              (`KismetSystemLibrary.Delay` 1.0)
              (goto _label)
              (else
                (`KismetArrayLibrary.Array_Clear` (`self.SpawnedEnemies`))
                (`self.SpawnEnemies`)))
            (else
              (`KismetSystemLibrary.Delay` 0.2)
              (`self.K2_DestroyActor`))))))))

(event `MultiCastCustomDepth`
  (params (Array :type "Array of Pawn Object Reference"))
  ;[0 0 0] Spawn AI.
  (if (`self.CustomDepthEnabled`)
    (for _array_element Array
      (message `/Game/ArcherySystem/Bow/BPI_BowPostProcess.EnableCustomDepth` _array_element))))

(fn `UserConstructionScript`)